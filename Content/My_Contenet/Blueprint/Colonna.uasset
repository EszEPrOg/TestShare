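; Colonna is a modular column Blueprint that resizes in height through the PrimaryColumn and SecondaryColumn variables.
; The construction script uses these variables as Z scales for two meshes, StaticMesh and StaticMesh2.
; It computes relative Z locations from those scales and fixed offsets to keep StaticMesh1, StaticMesh2 and StaticMesh3 stacked as the sections stretch.
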(fn `UserConstructionScript`
  (bind _staticmesh2 (`self.StaticMesh2`))
  (bind _secondary_column (`self.Secondary Column`))
  (bind _primary_column (`self.Primary Column`))
  (bind _returnvalue (* 100 _primary_column))
  (bind _returnvalue_2 (+ _returnvalue 100.0))
  (`SceneComponent.SetRelativeScale3D` (`self.StaticMesh`) (`KismetMathLibrary.MakeVector` 1.0 1.0 _primary_column))
  (`SceneComponent.K2_SetRelativeLocation` (`self.StaticMesh1`) (`KismetMathLibrary.MakeVector` 0.0 0.0 _returnvalue_2) false false)
  (`SceneComponent.K2_SetRelativeLocation` _staticmesh2 (`KismetMathLibrary.MakeVector` 0.0 0.0 (+ _returnvalue_2 7.0)) false false)
  (`SceneComponent.SetRelativeScale3D` _staticmesh2 (`KismetMathLibrary.MakeVector` 1.0 1.0 _secondary_column))
  (`SceneComponent.K2_SetRelativeLocation` (`self.StaticMesh3`) (`KismetMathLibrary.MakeVector` 0.0 0.0 (+ (+ (* 93 _secondary_column) _returnvalue) 107.0)) false false))